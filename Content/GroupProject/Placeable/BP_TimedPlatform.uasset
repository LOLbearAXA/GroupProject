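; BP_TimedPlatform is a placeable platform that falls and rises again in response to the main character.
; Entering its CollisionBox starts the FallingTime timeline after a Duration delay, and leaving it starts a second timeline for the rise after the same delay.
; Each timeline adds its Distance value as a local Z offset on every update, so movement accumulates per tick rather than interpolating between fixed positions.
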(event OnComponentBeginOverlap(CollisionBox)
  (params (OverlappedComponent :type Primitive%20Component%20Object%20Reference) (OtherActor :type Actor%20Object%20Reference) (OtherComp :type Primitive%20Component%20Object%20Reference) (OtherBodyIndex :type Integer) (bFromSweep :type Boolean) (SweepResult :type Hit%20Result%20Structure%20%28by%20ref%29))
  (bind _asbp_main_character (Utilities|Casting|CastToBP_MainCharacter OtherActor))
  (if (Utilities|IsValid _asbp_main_character)
    (Utilities|FlowControl|Delay (Variables|Default|GetDuration))
    (CallFunction|PlatformFalling)))

(event OnComponentEndOverlap(CollisionBox)
  (params (OverlappedComponent :type Primitive%20Component%20Object%20Reference) (OtherActor :type Actor%20Object%20Reference) (OtherComp :type Primitive%20Component%20Object%20Reference) (OtherBodyIndex :type Integer))
  (bind _asbp_main_character (Utilities|Casting|CastToBP_MainCharacter OtherActor))
  (if (Utilities|IsValid _asbp_main_character)
    (Utilities|FlowControl|Delay (Variables|Default|GetDuration))
    (CallFunction|RisePlatform)))

(event Custom|PlatformFalling
  (bind _distance (Timeline|FallingTime PlayFromStart)
    (:Update
      (Transformation|AddActorLocalOffset self (Math|Vector|MakeVector 0.0 0.0 _distance) false false))))

(event Custom|RisePlatform
  (bind _distance (Timeline|Timeline PlayFromStart)
    (:Update
      (Transformation|AddActorLocalOffset self (Math|Vector|MakeVector 0.0 0.0 _distance) false false))))

(fn ConstructionScript
  (|CallParentFunction))