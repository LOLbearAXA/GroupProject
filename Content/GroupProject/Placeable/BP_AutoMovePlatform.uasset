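; BP_AutoMovePlatform is a placeable platform that shuttles forward and back continuously from BeginPlay.
; Two timelines, GoingForward and GoingBack, trigger each other on finish, with RepeatTheMove restarting the cycle.
; Each update adds an unswept world offset of MovementSpeed along the actor's yaw-only forward vector, negated on return.
; The offset is not scaled by delta time, so travel distance depends on update count.
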(event Custom|RepeatTheMove
  (bind _self self)
  (bind _returnvalue (Transformation|GetActorRotation _self))
  (bind _returnvalue_2 (Math|Rotator|MakeRotator 0.0 0.0 (.yaw _returnvalue)))
  (bind _returnvalue_3 (Math|Vector|GetForwardVector _returnvalue_2))
  (Timeline|GoingForward PlayFromStart
    (:Update
      (Transformation|AddActorWorldOffset (* (Variables|Default|GetMovementSpeed) _returnvalue_3)))
    (:Finished
      (Timeline|GoingBack PlayFromStart
        (:Update
          (Transformation|AddActorWorldOffset (Math|Vector|NegateVector (* (Variables|Default|GetMovementSpeed) _returnvalue_3))))
        (:Finished
          (CallFunction|RepeattheMove))))))

(event EventBeginPlay
  (bind _self self)
  (bind _returnvalue (Transformation|GetActorRotation _self))
  (bind _returnvalue_2 (Math|Rotator|MakeRotator 0.0 0.0 (.yaw _returnvalue)))
  (bind _returnvalue_3 (Math|Vector|GetForwardVector _returnvalue_2))
  (Timeline|GoingForward Play
    (:Update
      (Transformation|AddActorWorldOffset (* (Variables|Default|GetMovementSpeed) _returnvalue_3)))
    (:Finished
      (Timeline|GoingBack PlayFromStart
        (:Update
          (Transformation|AddActorWorldOffset (Math|Vector|NegateVector (* (Variables|Default|GetMovementSpeed) _returnvalue_3))))
        (:Finished
          (CallFunction|RepeattheMove))))))

(fn ConstructionScript
  (|CallParentFunction))