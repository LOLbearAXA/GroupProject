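; BP_TurtorialText is a placeable actor that shows tutorial text in the world through a widget component.
; On BeginPlay it casts the widget to WBP_TurtorialText and passes it the Text variable through UpdateText.
; Every Tick it turns the widget toward player 0's camera on yaw only, applying the world-space look-at yaw as a relative rotation.
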(event EventBeginPlay
  ;[0.15 0.15 0.15 0.5] Update text
  (bind _aswbp_turtorial_text (Utilities|Casting|CastToWBP_TurtorialText (UserInterface|GetWidget (Variables|Default|GetWidget))))
  (Default|UpdateText _aswbp_turtorial_text (Variables|Default|GetText)))

(event EventTick
  (params (DeltaSeconds :type Float%20%28single-precision%29))
  ;[0.15 0.15 0.15 0.5] Make Widget face to player
  (Transformation|SetRelativeRotation (Variables|Default|GetWidget) (Math|Rotator|MakeRotator 0.0 0.0 (.yaw (Math|Rotator|FindLookatRotation (Transformation|GetWorldLocation (Variables|Default|GetWidget)) (Camera|GetCameraLocation (Game|GetPlayerCameraManager 0))))) false false))

(fn ConstructionScript
  (|CallParentFunction))