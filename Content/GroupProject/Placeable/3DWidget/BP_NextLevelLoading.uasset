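; BP_NextLevelLoading is a placeable trigger with a floating loading-bar widget for a next-level transition.
; On BeginPlay it passes the display text and level to WBP_FloatingUI_Loading and empties the bar.
; Player overlap with the collision box plays a timeline that drives the bar, and leaving reverses it.
; Tick yaws the widget toward the camera; no level loading happens in this Blueprint itself.
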(event OnComponentBeginOverlap(CollisionBox1)
  (params (OverlappedComponent :type Primitive%20Component%20Object%20Reference) (OtherActor :type Actor%20Object%20Reference) (OtherComp :type Primitive%20Component%20Object%20Reference) (OtherBodyIndex :type Integer) (bFromSweep :type Boolean) (SweepResult :type Hit%20Result%20Structure%20%28by%20ref%29))
  (if (== OtherActor (Game|GetPlayerCharacter 0))
    (bind _loadtime (Timeline|LoadingTIme Play)
      (:Update
        (Default|UpdateBar (Variables|Default|GetWidgetInUse) _loadtime)))))

(event OnComponentEndOverlap(CollisionBox1)
  (params (OverlappedComponent :type Primitive%20Component%20Object%20Reference) (OtherActor :type Actor%20Object%20Reference) (OtherComp :type Primitive%20Component%20Object%20Reference) (OtherBodyIndex :type Integer))
  (if (== OtherActor (Game|GetPlayerCharacter 0))
    (bind _loadtime (Timeline|LoadingTIme Reverse)
      (:Update
        (Default|UpdateBar (Variables|Default|GetWidgetInUse) _loadtime)))))

(event EventTick
  (params (DeltaSeconds :type Float%20%28single-precision%29))
  ;[0.15 0.15 0.15 0.5] Make Widget face to player
  (Transformation|SetRelativeRotation (Variables|Default|GetWidget) (Math|Rotator|MakeRotator 0.0 0.0 (.yaw (Math|Rotator|FindLookatRotation (Transformation|GetWorldLocation (Variables|Default|GetWidget)) (Camera|GetCameraLocation (Game|GetPlayerCameraManager 0))))) false false))

(event EventBeginPlay
  ;[0.15 0.15 0.15 0.5] Set Level and Text
  (bind _aswbp_floating_ui_loading (Utilities|Casting|CastToWBP_FloatingUI_Loading (UserInterface|GetWidget (Variables|Default|GetWidget))))
  (bind _output_get (Variables|Default|SetWidgetInUse _aswbp_floating_ui_loading))
  (Default|SetDisplayText _output_get (Variables|Default|GetDisplay%20Text))
  (Variables|/Game/GroupProject/UI/NextLevel3DWidget/WBP_FloatingUI_Loading.WBP_FloatingUI_Loading_C|SetLevel _output_get (Variables|Default|GetLevel))
  (Default|UpdateBar _output_get 0.0))

(fn ConstructionScript
  (|CallParentFunction))