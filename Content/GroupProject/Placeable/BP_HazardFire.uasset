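; BP_HazardFire is a placeable fire hazard that deals damage over time to the main character while they stand in it.
; Box begin overlap casts to BP_MainCharacter and starts a looping timer whose BurningDamage event calls CharacterOverlap, reducing health through UpdateHealth.
; Any end overlap on the box clears the timer, without checking which actor left.
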(event OnComponentBeginOverlap(Box)
  (params (OverlappedComponent :type Primitive%20Component%20Object%20Reference) (OtherActor :type Actor%20Object%20Reference) (OtherComp :type Primitive%20Component%20Object%20Reference) (OtherBodyIndex :type Integer) (bFromSweep :type Boolean) (SweepResult :type Hit%20Result%20Structure%20%28by%20ref%29))
  (bind _asbp_main_character (Utilities|Casting|CastToBP_MainCharacter OtherActor))
  (bind _returnvalue (Utilities|Time|SetTimerbyEvent (delegate Custom|BurningDamage) 1.0 true))
  (Variables|Default|SetTimerHandle _returnvalue))

(event OnComponentEndOverlap(Box)
  (params (OverlappedComponent :type Primitive%20Component%20Object%20Reference) (OtherActor :type Actor%20Object%20Reference) (OtherComp :type Primitive%20Component%20Object%20Reference) (OtherBodyIndex :type Integer))
  (Utilities|Time|ClearandInvalidateTimerbyHandle (Variables|Default|GetTimerHandle)))

(event Custom|BurningDamage
  (CallFunction|CharacterOverlap (stale OnComponentBeginOverlap(Box) _asbp_main_character)))

(fn ConstructionScript
  (|CallParentFunction))

(fn CharacterOverlap
  (params (CharacterRef :type BP%20Main%20Character%20Object%20Reference))
  (Default|UpdateHealth CharacterRef -2))