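; BP_HealthPickup is a placeable pickup that restores health to the character that overlaps it.
; CharacterOverlap skips characters already at max health; otherwise it calls UpdateHealth on the character with a fixed amount.
; It then deactivates its idle FXSHealthPickUp effect, spawns a collected effect at that spot and destroys itself.
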(event EventBeginPlay)

(event Collision|EventActorBeginOverlap
  (params (OtherActor :type Actor%20Object%20Reference)))

(event EventTick
  (params (DeltaSeconds :type Float%20%28single-precision%29)))

(fn ConstructionScript
  (|CallParentFunction))

(fn CharacterOverlap
  (params (CharacterRef :type BP%20Main%20Character%20Object%20Reference))
  (bind _fxs_healthpickup (Variables|Default|GetFXS_HealthPickUp))
  (if (not (== (Variables|/Game/GroupProject/Character/BP_MainCharacter.BP_MainCharacter_C|GetHealth CharacterRef) (Variables|/Game/GroupProject/Character/BP_MainCharacter.BP_MainCharacter_C|GetMaxHealth CharacterRef)))
    (Default|UpdateHealth CharacterRef 3)
    (Components|Activation|Deactivate _fxs_healthpickup)
    (Niagara|SpawnSystematLocation "/Game/GroupProject/VFX/FXS_HealthPickUpCollected.FXS_HealthPickUpCollected" (Transformation|GetWorldLocation _fxs_healthpickup))
    (Actor|DestroyActor)))